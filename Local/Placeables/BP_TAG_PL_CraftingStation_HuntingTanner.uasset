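; Placeable hunting tanner crafting station that exposes its first thrall inventory as the artisan thrall inventory.
; On BeginPlay it runs the parent logic, sends a placeholder-style text notification to its owner and binds to the placeable inventory's item-added signal.
; Each added item triggers SetupData to refresh the station, while the construction script only calls its parent.
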(event Custom|Notify
  (params (index :type Integer) (item :type Game%20Item%20Object%20Reference) (srcInventory :type Item%20Inventory%20Object%20Reference) (srcIndex :type Integer))
  (CallFunction|SetupData))

(event EventBeginPlay
  (|CallParentFunction)
  (Class|HUDNotificationInterface|NotificationText(Message) (Components|GetOwner) "mmmmm put it in me" false)
  (EventDispatchers|BindEventtoSignalItemAdded (Variables|Default|GetPlaceableInventory) (delegate Custom|Notify)))

(event Collision|EventActorBeginOverlap
  (params (OtherActor :type Actor%20Object%20Reference)))

(event EventTick
  (params (DeltaSeconds :type Float%20%28single-precision%29)))

(fn ConstructionScript
  (|CallParentFunction))

(fn GetArtisanThrallInventory
  (return (Variables|Default|GetThrallInventory_1)))