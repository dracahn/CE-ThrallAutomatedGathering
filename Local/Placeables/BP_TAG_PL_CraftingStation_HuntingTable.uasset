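; Hunting Table crafting station placeable that sizes its crafting queue by the hunter thralls placed in it.
; When an item is added to the placeable inventory, it recounts Archer and Fighter thralls with valid humanoid NPC spawn-table entries.
; That count, capped at MaxQueue, becomes the crafting queue's maximum item count.
; Only the item-added signal is bound here, and HelloWorld is a debug notification stub.
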(event Custom|Notify
  (params (index :type Integer) (item :type Game%20Item%20Object%20Reference) (srcInventory :type Item%20Inventory%20Object%20Reference) (srcIndex :type Integer))
  (CallFunction|SetupHunters))

(event EventBeginPlay
  (|CallParentFunction)
  (EventDispatchers|BindEventtoSignalItemAdded (Variables|Default|GetPlaceableInventory) (delegate Custom|Notify)))

(event Collision|EventActorBeginOverlap
  (params (OtherActor :type Actor%20Object%20Reference)))

(event EventTick
  (params (DeltaSeconds :type Float%20%28single-precision%29)))

(fn ConstructionScript
  (|CallParentFunction))

(fn GetArtisanThrallInventory
  (return (Variables|Default|GetThrallInventory)))

(fn HelloWorld
  (Class|HUDNotificationInterface|NotificationText(Message) self "Hello World" false))

(fn SetupHunters
  (Variables|Default|SetHunterThrallCount 0)
  (for _array_element (Variables|/Script/ConanSandbox.ItemInventory|GetItemList (Variables|Default|GetPlaceableInventory))
    ;[1 0.6413 0.1882] Validation
    (Utilities|IsValid _array_element ; Is the item a valid object
      (:Is%20Valid
        (bind _asthrall_item (Utilities|Casting|CastToThrallItem _array_element))
        (bind _returnvalue (Utilities|GetDataTableRow "/Game/Systems/SpawnTable/SpawnDataTable.SpawnDataTable" (.spawntableid (Variables|/Script/ConanSandbox.ThrallItem|GetThrallInfo _asthrall_item)))
          (:then
            (if (Utilities|IsValidClass (Utilities|ResolveSoftReference (.npcclass _returnvalue)))
              (Utilities|Casting|CastToBaseHumanoidNPCClass (Utilities|ResolveSoftReference (.npcclass _returnvalue)))
              (switch Utilities|FlowControl|Switch|SwitchonEThrallProfession (.thrallprofession (Variables|/Script/ConanSandbox.ThrallItem|GetThrallInfo _asthrall_item))
                (:Archer
                  _)
                (:Fighter
                  _))
              (Math|Integer|IncrementInt (Variables|Default|GetHunterThrallCount))))))))
  (CallFunction|SetupQueue))

(fn SetupQueue
  (if (> (Variables|Default|GetHunterThrallCount) (Variables|Default|GetMaxQueue))
    (LocalVariables|SetLocalQueue (Variables|Default|GetMaxQueue))
    (else
      (LocalVariables|SetLocalQueue (Variables|Default|GetHunterThrallCount))))
  (Class|ItemInventory|SetMaxItemCount (Variables|Default|GetCraftingQueue) (LocalVariables|GetLocalQueue)))