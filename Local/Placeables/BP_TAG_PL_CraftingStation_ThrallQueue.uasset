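; Crafting station placeable whose crafting queue capacity depends on the hunter thralls stored in its inventory.
; Inventory changes, client inventory receipt and completed crafts trigger a recount of Archer and Fighter thrall items with humanoid NPC classes in their spawn table rows.
; That count, capped by MaxQueue, sets the queue's maximum item count, and shrinking the queue clears all queued recipes.
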(event Custom|Notify
  (params (index :type Integer) (item :type Game%20Item%20Object%20Reference) (srcInventory :type Item%20Inventory%20Object%20Reference) (srcIndex :type Integer))
  (CallFunction|SetupHunters))

(event Custom|ItemCrafted
  (params (recipeItem :type Recipe%20Item%20Object%20Reference) (gameItem :type Game%20Item%20Object%20Reference) (stackSize :type Integer))
  (CallFunction|SetupHunters))

(event Custom|InventoryRecievedOnClient
  (CallFunction|SetupHunters))

(event EventBeginPlay
  (bind _placeableinventory (Variables|Default|GetPlaceableInventory))
  (|CallParentFunction)
  (Variables|Default|SetMaxQueue 5)
  (EventDispatchers|BindEventtoSignalItemAdded _placeableinventory (delegate Custom|Notify))
  (EventDispatchers|BindEventtoSignalItemRemoved _placeableinventory (delegate Custom|Notify))
  (EventDispatchers|BindEventtoSignalInventoryRecivedonClient _placeableinventory (delegate Custom|InventoryRecievedOnClient))
  (EventDispatchers|BindEventtoSignalItemCrafted (Variables|Default|GetCraftingQueue) (delegate Custom|ItemCrafted)))

(event Collision|EventActorBeginOverlap
  (params (OtherActor :type Actor%20Object%20Reference)))

(event EventTick
  (params (DeltaSeconds :type Float%20%28single-precision%29)))

(fn ConstructionScript
  (|CallParentFunction))

(fn GetArtisanThrallInventory
  (return 0))

(fn SetupHunters
  (bind _placeableinventory (Variables|Default|GetPlaceableInventory))
  (bind _itemlist (Variables|/Script/ConanSandbox.ItemInventory|GetItemList _placeableinventory))
  (Variables|Default|SetHunterThrallCount 0)
  (if (>= 100 (Utilities|Array|Length _itemlist))
    (for _array_element _itemlist
      ;[1 0.6413 0.1882] Validation
      (Utilities|IsValid _array_element ; Is the item a valid object
        (:Is%20Valid
          (bind _asthrall_item (Utilities|Casting|CastToThrallItem _array_element))
          (bind _returnvalue (Utilities|GetDataTableRow "/Game/Systems/SpawnTable/SpawnDataTable.SpawnDataTable" (.spawntableid (Variables|/Script/ConanSandbox.ThrallItem|GetThrallInfo _asthrall_item)))
            (:then
              (if (Utilities|IsValidClass (Utilities|ResolveSoftReference (.npcclass _returnvalue)))
                (Utilities|Casting|CastToBaseHumanoidNPCClass (Utilities|ResolveSoftReference (.npcclass _returnvalue)))
                (switch Utilities|FlowControl|Switch|SwitchonEThrallProfession (.thrallprofession (Variables|/Script/ConanSandbox.ThrallItem|GetThrallInfo _asthrall_item))
                  (:Archer
                    _)
                  (:Fighter
                    _))
                (Math|Integer|IncrementInt (Variables|Default|GetHunterThrallCount)))))))))
  (CallFunction|SetupQueue))

(fn SetupQueue
  (bind _craftingqueue (Variables|Default|GetCraftingQueue))
  (if (> (Variables|Default|GetHunterThrallCount) (Variables|Default|GetMaxQueue))
    (LocalVariables|SetLocalQueue (Variables|Default|GetMaxQueue))
    (else
      (LocalVariables|SetLocalQueue (Variables|Default|GetHunterThrallCount))))
  (if (> (Variables|/Script/ConanSandbox.ItemInventory|GetMaxItemCount _craftingqueue) (LocalVariables|GetLocalQueue)) ; If we're downsizing the queue
    (Class|CraftingQueue|RemoveAllRecipes _craftingqueue) ; Clear the queue
  )
  (Class|ItemInventory|SetMaxItemCount _craftingqueue (LocalVariables|GetLocalQueue)))