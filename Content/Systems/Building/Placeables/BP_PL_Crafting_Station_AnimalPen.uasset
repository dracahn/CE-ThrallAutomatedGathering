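; Animal pen crafting station placeable that displays the pets in its inventory as idle-animated skeletal meshes in five slots.
; Inventory changes and client replication rebuild per-slot meshes, animations, materials and rest sounds from each thrall item's spawn-table NPC class defaults, async loading classes as needed.
; Outside dedicated servers, an inventory monitor shows pets before any interaction, and a looping timer plays pet sounds, skipping a play while a sound loads.
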(event Custom|UpdatePetVisuals
  (params (index :type Integer) (item :type Game%20Item%20Object%20Reference) (dstInventory :type Item%20Inventory%20Object%20Reference) (dstIndex :type Integer))
  ;[1 0.6413 0.1882] [Set Pet Mesh Data]
  (Utilities|Casting|CastToThrallItemClass (Utilities|GetClass item))
  (CallFunction|SetupData))

(event Custom|AsyncLoadMeshes
  (params (Asset :type Conan%20Character%20Object%20Reference) (Index :type Integer))
  ;[0.02499 0.09524 0.16] [Async Load Meshes] If Necessary
  (bind _class (Utilities|AsyncLoadClassAsset Asset))
  (CallFunction|SetupDataInternal (Class|DreamworldBlueprints|GetClassDefaultObject _class) Index)
  (CallFunction|OnPetMeshDataReady))

(event Custom|PlayPetSounds
  ;[1 0.6413 0.1882] [Play Pet Sounds]
  (for (_array_element _array_index) (Variables|Default|GetPetSoundCues)
    (Utilities|IsAssetValid _array_element
      (:IsValid
        (Utilities|IsValid (Utilities|ResolveSoftReference _array_element)
          (:Is%20Valid
            (Audio|PlaySoundatLocation (Utilities|ResolveSoftReference _array_element) (Transformation|GetWorldLocation (Utilities|Array|Get(acopy) (Variables|Default|GetPets) _array_index))))
          (:Is%20Not%20Valid
            ;;[0.02499 0.09524 0.16] Don't play the this time around, and just load it instead.
            ;; To prevent desyncing sound effect length and loop time.
            (CallFunction|AsyncLoadSound _array_element)))))))

(event Custom|OnPetMeshDataReady
  ;[1 0.6413 0.1882] [On Pet Mesh Data Ready]
  (CallFunction|SetPetVisuals))

(event Custom|AsyncLoadSound
  (params (SoundCue :type Sound%20Cue%20Object%20Reference))
  ;[0.02499 0.09524 0.16] [Async Load Sound]
  (|LoadAssetsAsync (Utilities|Array|MakeArray SoundCue)))

(event Custom|InventoryRecievedOnClient
  ;[1 0.6413 0.1882] [Update Pet Mesh Data When Inventory Is Recieved On Client]
  (CallFunction|SetupData))

(event EventBeginPlay
  (bind _petinventory (Variables|Default|GetPetInventory))
  (|CallParentFunction)
  (Utilities|FlowControl|Sequence
    (:then_0
      (Utilities|FlowControl|Sequence
        (:then_0
          ;[0.02499 0.09524 0.16] Initialize Array for ease of access to components.
          (Variables|Default|SetPets (Utilities|Array|MakeArray (Variables|Default|GetPetSlot01) (Variables|Default|GetPetSlot02) (Variables|Default|GetPetSlot03) (Variables|Default|GetPetSlot04) (Variables|Default|GetPetSlot05)))
          (Utilities|Array|Resize (Variables|Default|GetPetIdleAnimations) 5)
          (Utilities|Array|Resize (Variables|Default|GetPetSkeletalMeshes) 5)
          (Utilities|Array|Resize (Variables|Default|GetPetSoundCues) 5))
        (:then_1
          ;[0.02499 0.09524 0.16] Bind Inventory Events
          (EventDispatchers|BindEventtoSignalItemAdded _petinventory (delegate Custom|UpdatePetVisuals))
          (EventDispatchers|BindEventtoSignalItemRemoved _petinventory (delegate Custom|UpdatePetVisuals))
          (EventDispatchers|BindEventtoSignalInventoryRecivedonClient _petinventory (delegate Custom|InventoryRecievedOnClient)))
        (:then_2
          ;[1 0.6413 0.1882] [Set Pet Mesh Data]
          (CallFunction|SetupData))
        (:then_3
          ;[1 0.6413 0.1882] [Play Pet Sounds]
          (if (not (Networking|IsDedicatedServer))
            (Utilities|Time|SetTimerbyEvent (delegate Custom|PlayPetSounds) 1e+01 true)))))
    (:then_1
      ;[0.02499 0.09524 0.16] Make sure that the pets show up even if the player hasn't interacted with the inventory.
      (if (not (Networking|IsDedicatedServer))
        (bind _returnvalue (Game|ConstructObjectfromClass "/Script/ConanSandbox.ItemInventoryClientMonitor" self))
        (Class|ItemInventoryClientMonitor|SetInventory _returnvalue (Variables|Default|GetPetInventory))))))

(event EventCleanUp
  ;[0.02499 0.09524 0.16] Override the Cleanup functionality so that it doesn't remove the PetSlots.
)

(fn ConstructionScript
  (|CallParentFunction))

(fn SetupDataInternal
  (params (ConanCharacter :type Conan%20Character%20Object%20Reference) (Index :type Integer))
  (LocalVariables|SetLocal_ConanCharacter ConanCharacter)
  (LocalVariables|SetLocal_Index Index)
  (Utilities|IsValid (LocalVariables|GetLocal_ConanCharacter)
    (:Is%20Valid
      ;[0.02499 0.09524 0.16] Set Array Element
      (bind _soundcue (CallFunction|GetRestSoundCue (LocalVariables|GetLocal_ConanCharacter)))
      (Utilities|Array|SetArrayElem (Variables|Default|GetPetSoundCues) (LocalVariables|GetLocal_Index) _soundcue true)
      (bind _asab_master_quadropeds (Utilities|Casting|CastToAB_Master_Quadropeds (Class|DreamworldBlueprints|GetClassDefaultObject (Variables|/Script/Engine.SkeletalMeshComponent|GetAnimClass (Variables|/Script/Engine.Character|GetMesh (LocalVariables|GetLocal_ConanCharacter))))))
      (Utilities|Array|SetArrayElem (Variables|Default|GetPetIdleAnimations) (LocalVariables|GetLocal_Index) (Variables|/Game/Master_AnimBP/AB_Master_Quadropeds.AB_Master_Quadropeds_C|GetIdleAnimalPen _asab_master_quadropeds) true)
      (Utilities|Array|SetArrayElem (Variables|Default|GetPetSkeletalMeshes) (LocalVariables|GetLocal_Index) (Variables|/Script/Engine.SkinnedMeshComponent|GetSkeletalMesh (Variables|/Script/Engine.Character|GetMesh (LocalVariables|GetLocal_ConanCharacter))) true)
      ;[0.02499 0.09524 0.16] Set Materials
      (for (_array_element _array_index) (Rendering|Material|GetMaterials (Variables|/Script/Engine.Character|GetMesh (LocalVariables|GetLocal_ConanCharacter)))
        (Rendering|Material|SetMaterial (Utilities|Array|Get(acopy) (Variables|Default|GetPets) (LocalVariables|GetLocal_Index)) _array_index _array_element)))
    (:Is%20Not%20Valid
      ;[0.02499 0.09524 0.16] Clear Array Element
      (Utilities|Array|SetArrayElem (Variables|Default|GetPetIdleAnimations) (LocalVariables|GetLocal_Index) 0 true)
      (Utilities|Array|SetArrayElem (Variables|Default|GetPetSkeletalMeshes) (LocalVariables|GetLocal_Index) 0 true)
      (Utilities|Array|SetArrayElem (Variables|Default|GetPetSoundCues) (LocalVariables|GetLocal_Index) 0 true))))

(fn SetupData
  (for (_array_element _array_index) (Variables|/Script/ConanSandbox.ItemInventory|GetItemList (Variables|Default|GetPetInventory))
    ;[1 0.6413 0.1882] Validation
    (Utilities|IsValid _array_element
      (:Is%20Valid
        (bind _asthrall_item (Utilities|Casting|CastToThrallItem _array_element))
        (bind _returnvalue (Utilities|GetDataTableRow "/Game/Systems/SpawnTable/SpawnDataTable.SpawnDataTable" (.spawntableid (Variables|/Script/ConanSandbox.ThrallItem|GetThrallInfo _asthrall_item)))
          (:then
            (if (Utilities|IsValidClass (Utilities|ResolveSoftReference (.npcclass _returnvalue)))
              (CallFunction|SetupDataInternal (Class|DreamworldBlueprints|GetClassDefaultObject (Utilities|ResolveSoftReference (.npcclass _returnvalue))) _array_index)
              (else
                (CallFunction|AsyncLoadMeshes (.npcclass _returnvalue) _array_index))))))
      (:Is%20Not%20Valid
        (CallFunction|SetupDataInternal 0 _array_index))))
  (CallFunction|OnPetMeshDataReady))

(fn SetPetVisuals
  ;[1 0.6413 0.1882] Set Skeletal Mesh
  (for (_array_element _array_index) (Variables|Default|GetPets)
    (if (Utilities|IsValid (Utilities|Array|Get(acopy) (Variables|Default|GetPetSkeletalMeshes) _array_index))
      (Class|SkinnedMeshComponent|SetSkeletalMesh _array_element (Utilities|Array|Get(acopy) (Variables|Default|GetPetSkeletalMeshes) _array_index) true)
      ;[1 0.6413 0.1882] Start Animations
      (Components|Animation|PlayAnimation _array_element (Utilities|Array|Get(acopy) (Variables|Default|GetPetIdleAnimations) _array_index) true)
      ;[1 0.6413 0.1882] Set Visibility
      (Rendering|SetVisibility _array_element (Utilities|IsValid (Utilities|Array|Get(acopy) (Variables|Default|GetPetSkeletalMeshes) _array_index)) true)
      (else
        (Class|SkinnedMeshComponent|SetSkeletalMesh _array_element 0 true)))))

(fn GetRestSoundCue
  (params (ConanCharacter :type Conan%20Character%20Object%20Reference))
  (bind _asbase_bpchar_interface (Utilities|Casting|CastToBaseBPCharInterface ConanCharacter)
    (:then
      (bind _voiceset (Default|GetVoiceSet _asbase_bpchar_interface))
      (Utilities|IsAssetValid (Class|AudioFunctionLibrary|GetVoiceSoundCue (Utilities|String|StringToName (Utilities|String|ToString(Text) (Utilities|Text|FormatText "{VoiceSet}_voc_rest_pen" (Utilities|Text|ToText(String) (Utilities|String|EnumtoString _voiceset))))) "VoiceSet")
        (:IsValid
          (return (Class|AudioFunctionLibrary|GetVoiceSoundCue (Utilities|String|StringToName (Utilities|String|ToString(Text) (Utilities|Text|FormatText "{VoiceSet}_voc_rest_pen" (Utilities|Text|ToText(String) (Utilities|String|EnumtoString _voiceset))))) "VoiceSet")))
        (:Is%20Not%20Valid
          (return 0))))
    (:CastFailed
      (return 0))))